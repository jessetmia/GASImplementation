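; Master gameplay ability for a primary combo attack, where each activation plays the montage mapped to the current combo count.
; Activation clears the pending timeout, and every montage exit (completed, blended out, interrupted or cancelled) ends the ability.
; That same exit then advances the count, or resets it after the last mapped attack, and starts a short timer that resets the combo unless the ability activates again.
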(event Custom|ComboTimeoutEvent
  (Variables|Default|SetCurrentComboCount 1)
  (Development|PrintString "Resetting combo!"))

(event Ability|EventActivateAbility
  (Utilities|Time|ClearandInvalidateTimerbyHandle (Variables|Default|GetComboTimeoutTimer))
  (|PlayMontageandWaitProxy "None" (.Value (Utilities|Map|Find (Variables|Default|GetAttackMontageComboMap) (Variables|Default|GetCurrentComboCount))) 1.0 "None" true 1.0 0.0 false
    (:OnCompleted
      _)
    (:OnBlendOut
      _)
    (:OnInterrupted
      _)
    (:OnCancelled
      _))
  (Ability|EndAbility)
  (Utilities|FlowControl|Sequence
    (:then_0
      (if (== (Variables|Default|GetCurrentComboCount) (Utilities|Map|Length (Variables|Default|GetAttackMontageComboMap)))
        (CallFunction|ComboTimeoutEvent)
        (else
          (Math|Integer|IncrementInt (Variables|Default|GetCurrentComboCount)))))
    (:then_1
      (bind _returnvalue (Utilities|Time|SetTimerbyEvent (delegate Custom|ComboTimeoutEvent) 0.5))
      (Variables|Default|SetComboTimeoutTimer _returnvalue))))