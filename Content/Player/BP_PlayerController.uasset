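; Player controller that toggles the in-game menu and a Steam friends list overlay, along with mouse cursor and input mode.
; Escape gets the main widget from HnSHUD, casts it to UI_StaminaBar, and shows or hides its menu based on its open state.
; BeginPlay creates the friends list hidden.
; F uses a FlipFlop to find and toggle it, independently of the menu state.
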(event EventBeginPlay
  (bind _returnvalue (UserInterface|CreateWidget "/Game/UI/Menu/Invite/UI_SteamFriendsList.UI_SteamFriendsList_C" (Game|GetPlayerController 0)))
  (Utilities|IsValid _returnvalue
    (:Is%20Valid
      (Widget|SetVisibility _returnvalue "Hidden")
      (UserInterface|Viewport|AddtoViewport _returnvalue 0))))

(event Input|KeyboardEvents|Escape
  (params (Key :type Key%20Structure :default "None"))
  (bind _returnvalue (Game|GetPlayerController 0))
  (:Pressed
    (bind _ashn_shud (Utilities|Casting|CastToHnSHUD (HUD|GetHUD (Game|GetPlayerController 0))))
    (bind _returnvalue_2 (Class|HnSHUD|GetMainWidget _ashn_shud))
    (Utilities|IsValid _returnvalue_2
      (:Is%20Valid
        (bind _asui_stamina_bar (Utilities|Casting|CastToUI_StaminaBar _returnvalue_2)
          (:then
            (bind _ismenuopened (Default|IsMenuOpened _asui_stamina_bar))
            (Variables|/Script/Engine.PlayerController|SetbShowMouseCursor _returnvalue (not _ismenuopened))
            (if _ismenuopened
              (Default|HideinGameMenu _asui_stamina_bar)
              (Input|SetInputModeGameOnly _returnvalue false)
              (else
                (Default|ShowinGameMenu _asui_stamina_bar)
                (Input|SetInputModeGameandUI _returnvalue _asui_stamina_bar "LockOnCapture" false false))))
          (:CastFailed
            (Development|PrintString "BITCH FAILED")))))))

(event Input|KeyboardEvents|F
  (params (Key :type Key%20Structure :default "None"))
  (bind _returnvalue (Game|GetPlayerController 0))
  (:Pressed
    (Utilities|FlowControl|FlipFlop
      (:A
        (bind _foundwidgets (Widget|GetAllWidgetsOfClass "/Game/UI/Menu/Invite/UI_SteamFriendsList.UI_SteamFriendsList_C" true))
        (Widget|SetVisibility _foundwidgets "Visible")
        (Variables|Default|SetbShowMouseCursor true)
        (Input|SetInputModeGameandUI _returnvalue 0 "DoNotLock" true false))
      (:B
        (bind _foundwidgets_2 (Widget|GetAllWidgetsOfClass "/Game/UI/Menu/Invite/UI_SteamFriendsList.UI_SteamFriendsList_C" true))
        (Widget|SetVisibility _foundwidgets_2 "Collapsed")
        (Variables|Default|SetbShowMouseCursor false)
        (Input|SetInputModeGameOnly _returnvalue false)))))

(fn ConstructionScript)